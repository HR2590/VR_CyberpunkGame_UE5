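; AC_RevealingObject is a component that links the shoot input to a BP_RevealGun for painting that reveals objects.
; SetRevealComponent caches the gun from a child actor component.
; While IA_Shoot triggers, it passes the camera's location and forward vector to the gun's paint dispatcher, up to a ray-count cap.
; Beyond the cap it calls paint recovery, as does release, which also resets the counter and clears stored collision UVs.
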(event `EnhancedInput|/Game/Core/Controls/IA_Shoot`
  (params (ActionValue :type Boolean) (ElapsedSeconds :type "Float (double-precision)") (TriggeredSeconds :type "Float (double-precision)") (InputAction :type "InputAction Object Reference" :default "/Game/Core/Controls/IA_Shoot.IA_Shoot"))
  (bind _returnvalue (`GameplayStatics.GetPlayerCameraManager` 0))
  (:`Triggered`
    (if (<= (`self.CounterRays`) 100)
      (`/Engine/EditorBlueprintResources/StandardMacros.IncrementInt` (`self.CounterRays`)
        (:`  `
          (`/Game/Core/RevealingGun/BP_RevealGun.PaintDispatcher` (`self.As BP Reveal Gun`) (`KismetMathLibrary.Conv_BoolToDouble` ActionValue) (`Actor.GetActorForwardVector` _returnvalue) (`Actor.K2_GetActorLocation` _returnvalue) null "None")))
      (else
        (`/Game/Core/RevealingGun/BP_RevealGun.RecoverPaint` (`self.As BP Reveal Gun`) :!label _label))))
  (:`Completed`
    (set `self.CounterRays` 0)
    (`KismetArrayLibrary.Array_Clear` (`/Game/Core/RevealingGun/BP_RevealGun.CollisionsUV` (`self.As BP Reveal Gun`)))
    (goto _label)))

(fn `SetRevealComponent`
  (params (RevealComponent :type "ChildActorComponent Object Reference"))
  (bind _asbp_reveal_gun (cast `/Game/Core/RevealingGun/BP_RevealGun` (`ChildActorComponent.ChildActor` RevealComponent)))
  (set `self.As BP Reveal Gun` _asbp_reveal_gun))