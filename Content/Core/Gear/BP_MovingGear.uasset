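; BP_MovingGear is a gear actor that keeps its mesh material's Direction parameter in step with back-and-forth travel between two points.
; BeginPlay caches the start position and computes the end point from GetTargetLocation as a relative offset.
; Tick pushes Direction to the materials, then sets it negative at the end point and positive at the start, using a small tolerance.
; The graph itself never moves the actor.
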(event `self.ReceiveBeginPlay`
  (bind _returnvalue (`self.K2_GetActorLocation`))
  (bind _returnvalue_2 (`self.GetTargetLocation`))
  (set `self.InitialPosition` _returnvalue)
  (set `self.AbsoluteFinalPosition` (+ _returnvalue_2 _returnvalue)))

(event `self.ReceiveTick`
  (params (DeltaSeconds :type "Float (single-precision)"))
  (bind _returnvalue (`self.K2_GetActorLocation`))
  (`MeshComponent.SetScalarParameterValueOnMaterials` (`self.StaticMesh`) "Direction" (`self.Direction`))
  (if (== (`self.AbsoluteFinalPosition`) _returnvalue :`ErrorTolerance` 1.0)
    (set `self.Direction` -1.0)
    (elif (== _returnvalue (`self.InitialPosition`) :`ErrorTolerance` 1.0)
      (set `self.Direction` 1.0))))

(fn `UserConstructionScript`)