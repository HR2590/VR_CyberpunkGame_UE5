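; Actor component that drives a BP_RevealGun from the IA_Shoot input.
; SetRevealComponent stores the gun and binds its paint event, and ClearRevealComponent unbinds and releases it.
; While shoot triggers, it fires the gun's paint dispatcher until a ray counter passes its cap or the gun's box simulates physics, then calls Recover instead.
; Releasing the input resets the counter.
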(event `EnhancedInput|/Game/Core/Controls/IA_Shoot`
  (params (ActionValue :type Boolean) (ElapsedSeconds :type "Float (double-precision)") (TriggeredSeconds :type "Float (double-precision)") (InputAction :type "InputAction Object Reference" :default "/Game/Core/Controls/IA_Shoot.IA_Shoot"))
  (:`Triggered`
    (if (!= (`self.As BP Reveal Gun`) null)
      (if (and (<= (`self.CounterRays`) 100) (not (`SceneComponent.IsSimulatingPhysics` (`/Game/Core/RevealingGun/BP_RevealGun.Box` (`self.As BP Reveal Gun`)) "None")))
        (`/Engine/EditorBlueprintResources/StandardMacros.IncrementInt` (`self.CounterRays`)
          (:`  `
            (`/Game/Core/RevealingGun/BP_RevealGun.PaintDispatcher` (`self.As BP Reveal Gun`) (`KismetMathLibrary.Conv_BoolToDouble` ActionValue))))
        (else
          (`/Game/Core/RevealingGun/BP_RevealGun.Recover` (`self.As BP Reveal Gun`))))))
  (:`Completed`
    (set `self.CounterRays` 0)))

(fn `ClearRevealComponent`
  (clear `/Game/Core/RevealingGun/BP_RevealGun.PaintDispatcher` (`self.As BP Reveal Gun`))
  (set `self.As BP Reveal Gun` null))

(fn `SetRevealComponent`
  (params (InActor :type "Actor Object Reference"))
  (if (!= (`self.As BP Reveal Gun`) InActor)
    (bind _asbp_reveal_gun (cast `/Game/Core/RevealingGun/BP_RevealGun` InActor))
    (bind _output_get (set `self.As BP Reveal Gun` _asbp_reveal_gun))
    (`/Game/Core/RevealingGun/BP_RevealGun.BindPaint` _output_get)))