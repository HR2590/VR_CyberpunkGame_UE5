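; BP_RevealGun is a paint gun that fires a Niagara reveal effect and shows a brush widget on screen.
; On paint input, unless the component is simulating physics, it runs a short line trace, unused downstream, and spawns attached particles.
; The particles report back through a Niagara callback, which currently only prints their positions.
; Brush drawing on BP_DoorHiding at hit UVs and the binding for texture recovery are disconnected.
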(event `Recover`
  (`/Game/BP_DoorHiding.ComeBackTexture` (`self.As BP Door Hiding`)))

(event `self.ReceiveBeginPlay`
  (bind _returnvalue (`|CreateWidget` "/Game/W_BrushToPaint.W_BrushToPaint_C"))
  (`UserWidget.AddToViewport` _returnvalue 0)
  (add `self.PaintDispatcher` (delegate `Paint`)))

(event `Paint` :!signature `self.PaintDispatcher`
  (params (ActionValue :type "Float (double-precision)") (TraceLine :type "Vector Structure") (ActorLocation :type "Vector Structure") (SceneComponent :type "SceneComponent Object Reference") (BoneName :type Name))
  (bind _arrow (`self.Arrow`))
  (if (`SceneComponent.IsSimulatingPhysics` SceneComponent BoneName)
    _
    (elif (== ActionValue 1.0)
      (`KismetSystemLibrary.LineTraceSingle` :`Start` ActorLocation :`End` (+ (`SceneComponent.K2_GetComponentLocation` _arrow) (* (`SceneComponent.GetForwardVector` _arrow) 150.0)) :`TraceChannel` "TraceTypeQuery1" :`bTraceComplex` true :`DrawTime` 1.0)
      (bind _returnvalue (`NiagaraFunctionLibrary.SpawnSystemAttached` "/Game/RevealParticles.RevealParticles" (`self.RevealParticles`) "None" (0.0 0.0 0.0) (struct) "KeepRelativeOffset" true))
      (bind _output_get (set `self.NiagaraSystem` _returnvalue))
      (`NiagaraComponent.SetNiagaraVariableObject` _output_get "User.BPCallBack" self))))

(event `self.ReceiveParticleData`
  (params (Data :type "Array of BasicParticleData Structure (by ref)") (NiagaraSystem :type "NiagaraSystem Object Reference") (SimulationPositionOffset :type "Vector Structure (by ref)"))
  (for _array_element Data
    (`KismetSystemLibrary.PrintString` (`KismetStringLibrary.Conv_VectorToString` (`.Position` (break `BasicParticleData` _array_element))))))

(fn `UserConstructionScript`)