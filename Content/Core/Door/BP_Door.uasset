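; Sliding door actor that splits vertically, moving one mesh up and another down when opened.
; Open and Close each play their own timeline, scaling the ZDirection track by per-mesh Z distances to set relative locations.
; When a timeline finishes, it updates IsOpened and clears IsOpeningOrClosing, which neither event sets or checks here.
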(event `self.Open`
  (bind (_direction _zdirection) (`Timeline|Timeline` :!via `PlayFromStart`)
    (:`Update`
      (`SceneComponent.K2_SetRelativeLocation` (`self.UpMovableMesh`) (`KismetMathLibrary.MakeVector` 0.0 0.0 (* _zdirection (`self.UpZDistance`))) false false)
      (`SceneComponent.K2_SetRelativeLocation` (`self.DownMovableMesh`) (`KismetMathLibrary.MakeVector` 0.0 0.0 (* _zdirection (* (`self.DownZDistance`) -1.0))) false false))
    (:`Finished`
      (set `self.bIsOpened` true)
      (set `self.bIsOpeningOrClosing` false))))

(event `self.Close`
  (bind _downzdistance (`self.DownZDistance`))
  (bind (_direction _zdirection) (`Timeline|Timeline_0` :!via `PlayFromStart`)
    (:`Update`
      (`SceneComponent.K2_SetRelativeLocation` (`self.UpMovableMesh`) (`KismetMathLibrary.MakeVector` 0.0 0.0 (- (`self.UpZDistance`) (* (`self.UpZDistance`) _zdirection))) false false)
      (`SceneComponent.K2_SetRelativeLocation` (`self.DownMovableMesh`) (`KismetMathLibrary.MakeVector` 0.0 0.0 (+ (* _zdirection _downzdistance) (* _downzdistance -1.0))) false false))
    (:`Finished`
      (set `self.bIsOpened` false)
      (set `self.bIsOpeningOrClosing` false))))

(fn `UserConstructionScript`)