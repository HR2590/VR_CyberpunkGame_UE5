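; Katana blade actor that cuts destructible objects its HitBox touches.
; On overlap start, it calls CutObject on BP_BaseDestructible actors, defining the cut plane from the HitBox's location and up vector.
; A DoOnce gate limits triggering until any overlap ends and resets it.
; Disconnected nodes retain an unused direct procedural-mesh slice and impulse approach.
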(event `self.HitBox.OnComponentBeginOverlap`
  (params (OverlappedComponent :type "PrimitiveComponent Object Reference") (OtherActor :type "Actor Object Reference") (OtherComp :type "PrimitiveComponent Object Reference") (OtherBodyIndex :type Integer) (bFromSweep :type Boolean) (SweepResult :type "HitResult Structure (by ref)"))
  (bind _hitbox (`self.HitBox`))
  (`/Engine/EditorBlueprintResources/StandardMacros.DoOnce` false :!label _label
    (:`Completed`
      (bind _asbp_base_destructible (cast `/Game/Core/Katana/BP_BaseDestructible` OtherActor))
      (`/Game/Core/Katana/BP_BaseDestructible.CutObject` _asbp_base_destructible (`SceneComponent.K2_GetComponentLocation` _hitbox) (`SceneComponent.GetUpVector` _hitbox)))))

(event `self.HitBox.OnComponentEndOverlap`
  (params (OverlappedComponent :type "PrimitiveComponent Object Reference") (OtherActor :type "Actor Object Reference") (OtherComp :type "PrimitiveComponent Object Reference") (OtherBodyIndex :type Integer))
  (goto _label :!via `Reset`))

(fn `UserConstructionScript`)