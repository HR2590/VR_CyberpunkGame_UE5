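; BP_ScannerComponent is a widget component that shows a scanner UI with info text from scanneable components.
; On BeginPlay it caches its UW_Scanner widget, and InfotoUI pushes a component's text into it and enables the info panel.
; Passing the currently scanned component again toggles the info off.
; ActivateScanner and DeactivateScanner set the component's visibility and both clear the text and current target.
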(event `self.ReceiveBeginPlay`
  (bind _asuw_scanner (cast `/Game/Core/Scanner/UserInterface/UW_Scanner` (`self.GetUserWidgetObject`)))
  (set `self.UWScannerObject` _asuw_scanner))

(event `self.InfoToUI`
  (params (ScanneableComponent :type "ScanneableComponent Object Reference"))
  (if (== ScanneableComponent (`self.CurrentScaningComponent`))
    (`self.ResetUIScannerObject`)
    (else
      (set `self.CurrentScaningComponent` ScanneableComponent)
      (bind _uwscannerobject (`self.UWScannerObject`)
        (:`then`
          (`/Game/Core/Scanner/UserInterface/UW_Scanner.Set Text From Info` _uwscannerobject (`ScanneableComponent.Text` (`self.CurrentScaningComponent`)))
          (`/Game/Core/Scanner/UserInterface/UW_Scanner.EnableInfoWidget` _uwscannerobject true))
        (:`else`)))))

(event `self.ActivateScanner`
  (`self.SetVisibility` true)
  (`self.ResetUIScannerObject`))

(event `self.DeactivateScanner`
  (`self.SetVisibility` false)
  (`self.ResetUIScannerObject`))

(fn `ResetUIScannerObject`
  (bind _uwscannerobject (`self.UWScannerObject`)
    (:`then`
      (`/Game/Core/Scanner/UserInterface/UW_Scanner.Set Text From Info` _uwscannerobject "")
      (`/Game/Core/Scanner/UserInterface/UW_Scanner.EnableInfoWidget` _uwscannerobject false)
      (set `self.CurrentScaningComponent` null))
    (:`else`)))